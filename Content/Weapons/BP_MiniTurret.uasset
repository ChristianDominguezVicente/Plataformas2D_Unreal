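; BP_MiniTurret is a turret that repeatedly spawns BP_EnemyBullet at its FirePoint transform, with no targeting logic.
; Tick drives firing through a CanFire gate, which closes on each shot and reopens after a FireTime delay.
; An unconnected node chain would slide the Shutter component backward along the actor's forward vector by ShutterMovement, but it never runs.
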(event `self.ReceiveBeginPlay`)

(event `self.ReceiveTick`
  (params (DeltaSeconds :type "Float (single-precision)"))
  (if (`self.CanFire`)
    (set `self.CanFire` false)
    (`|SpawnActorFromClass` "/Game/Weapons/BP_EnemyBullet.BP_EnemyBullet_C" (`SceneComponent.K2_GetComponentToWorld` (`self.FirePoint`)) "Undefined" "MultiplyWithRoot" null null)
    (`KismetSystemLibrary.Delay` (`self.FireTime`))
    (set `self.CanFire` true)))

(fn `UserConstructionScript`)