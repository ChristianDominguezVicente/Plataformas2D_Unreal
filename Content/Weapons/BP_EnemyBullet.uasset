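; Enemy bullet actor that flies straight ahead and damages the player character on overlap.
; Tick moves it along its forward vector at constant speed, scaled by delta time and without sweeping.
; Overlapping BP_ThirdPersonCharacter applies fixed damage with the bullet as causer, then destroys it.
; Any other overlap also destroys it, and a timer started on BeginPlay removes it after a few seconds.
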(event `self.ReceiveBeginPlay`
  ;[1 1 1] Timer de destrucción
  (`KismetSystemLibrary.K2_SetTimerDelegate` (delegate `Destroy`) 3.0))

(event `Destroy`
  ;[1 1 1] Timer de destrucción
  (`self.K2_DestroyActor` :!label _label))

(event `self.ReceiveActorBeginOverlap`
  (params (OtherActor :type "Actor Object Reference"))
  ;[1 1 1] Entrar en contacto con el player
  (bind _asbp_third_person_character (cast `/Game/ThirdPerson/Blueprints/BP_ThirdPersonCharacter` OtherActor)
    (:`then`
      (`GameplayStatics.ApplyDamage` _asbp_third_person_character 10.0 null self)
      (`self.K2_DestroyActor`))
    (:`CastFailed`
      (goto _label))))

(event `self.ReceiveTick`
  (params (DeltaSeconds :type "Float (single-precision)"))
  ;[1 1 1] Movimiento de las balas
  (`self.K2_SetActorLocation` (+ (`self.K2_GetActorLocation`) (* (* DeltaSeconds 1000.0) (`self.GetActorForwardVector`)))))

(fn `UserConstructionScript`)